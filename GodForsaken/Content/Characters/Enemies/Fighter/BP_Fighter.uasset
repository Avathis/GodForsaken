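; BP_Fighter is the Blueprint for the Fighter enemy character, built on the Gameplay Ability System.
; On BeginPlay it grants itself hit, punch and combo abilities, then applies a poise regeneration gameplay effect.
; The graph has no Tick or overlap logic, and leftover poise-printing and gameplay-event nodes are disconnected.
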(event `self.ReceiveBeginPlay`
  (`self.GrantAbility` "/Game/Characters/GeneralEventAbilities/Hit/GA_Hit.GA_Hit_C")
  (`self.GrantAbility` "/Game/Characters/Enemies/Fighter/Abilities/GA_FighterPunch.GA_FighterPunch_C")
  (`self.GrantAbility` "/Game/Characters/Enemies/Fighter/Abilities/GA_FighterCombo.GA_FighterCombo_C")
  (`AbilitySystemComponent.BP_ApplyGameplayEffectToSelf` :`self` (`self.AbilitySystemComponent`) :`GameplayEffectClass` "/Game/Characters/GE_PoiseRegen.GE_PoiseRegen_C"))

(event `self.ReceiveTick`
  (params (DeltaSeconds :type "Float (single-precision)")))

(fn `UserConstructionScript`)