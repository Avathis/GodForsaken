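; BP_Splash_Decal is a splash decal actor from an explosion VFX pack that fades out and destroys itself.
; The construction script applies the configured decal material and fade timing.
; On BeginPlay it adds a random roll, then creates a dynamic material instance with a randomized TextureLifetime parameter, so each splash varies in orientation and appearance.
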(event `self.ReceiveBeginPlay`
  (`self.K2_AddActorLocalRotation` (`KismetMathLibrary.MakeRotator` (`KismetMathLibrary.RandomFloatInRange` 0.0 360.0)))
  (bind _returnvalue (`DecalComponent.CreateDynamicMaterialInstance` (`self.Decal`)))
  (set `self.DynMat` _returnvalue)
  (`MaterialInstanceDynamic.SetScalarParameterValue` (`self.DynMat`) "TextureLifetime" (`KismetMathLibrary.RandomFloatInRange` 0.0 0.3)))

(fn `UserConstructionScript`
  (`DecalComponent.SetDecalMaterial` (`self.Decal`) (`self.DecalMaterial`))
  (`DecalComponent.SetFadeOut` (`self.Decal`) (`self.Start Delay`) (`self.Duration`) true))